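; Logger component that records its owner's movement and the camera's orientation to a timestamped, semicolon-separated log file during play.
; BeginPlay starts a looping timer at LogFrequency that appends location, camera rotation, up and forward vectors, FPS and timestamp.
; Tick sets FPS using modulo (1.0 % DeltaSeconds) rather than division.
; LogData optionally saves viewport screenshots every SkipFrames samples; StopLogging only clears IsLogging, leaving the timer uncleared.
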(event EventBeginPlay
  (bind _returnvalue (Game|GetPlayerController 0))
  (bind (_sizex _sizey) (HUD|GetViewportSize _returnvalue))
  (if (Variables|Default|GetUseDefaultSize)
    (Variables|Default|SetScreenSizeX _sizex)
    (Variables|Default|SetScreenSizeY _sizey))
  (Variables|Default|SetCameraManager (Game|GetPlayerCameraManager 0))
  (Variables|Default|SetActor (Components|GetOwner))
  (CallFunction|StartLogging))

(event EventTick
  (params (DeltaSeconds :type Float%20%28single-precision%29))
  (Variables|Default|SetFPS (Math|Float|%(Float) 1.0 DeltaSeconds)))

(event EventEndPlay
  (params (EndPlayReason :type EEndPlayReason%20Enum :default "Destroyed"))
  (CallFunction|StopLogging))

(fn LogData
  (bind _actor (Variables|Default|GetActor))
  (bind _cameramanager (Variables|Default|GetCameraManager))
  (bind _returnvalue (Transformation|GetActorLocation _actor))
  (bind _returnvalue_2 (Camera|GetCameraRotation _cameramanager))
  (bind _returnvalue_3 (Math|Vector|GetForwardVector _returnvalue_2))
  (bind _returnvalue_4 (Math|Vector|GetUpVector _returnvalue_2))
  (bind (_x _y _z) (Math|Vector|BreakVector _returnvalue))
  (bind (_roll _pitch _yaw) (Math|Rotator|BreakRotator _returnvalue_2))
  (bind (_x_2 _y_2 _z_2) (Math|Vector|BreakVector _returnvalue_4))
  (bind (_x_3 _y_3 _z_3) (Math|Vector|BreakVector _returnvalue_3))
  (bind _output_get (LocalVariables|SetNow (Math|DateTime|Now)))
  (bind _returnvalue_5 (Class|LoggingBlueprintFunctionLibrary|GetDateTimeString _output_get))
  (LocalVariables|SetDateTimeString _returnvalue_5)
  (Class|LoggingBlueprintFunctionLibrary|AppendLogtoFile (Utilities|String|Append (Utilities|String|Append (Utilities|String|ToString(Float) _x) ";" (Utilities|String|ToString(Float) _y) ";" (Utilities|String|ToString(Float) _z) ";" (Utilities|String|ToString(Float) _roll) ";" (Utilities|String|ToString(Float) _pitch) ";" (Utilities|String|ToString(Float) _yaw) ";" (Utilities|String|ToString(Float) _x_2) ";" (Utilities|String|ToString(Float) _y_2) ";" (Utilities|String|ToString(Float) _z_2) ";" (Utilities|String|ToString(Float) _x_3) ";" (Utilities|String|ToString(Float) _y_3) ";" (Utilities|String|ToString(Float) _z_3) ";") (Utilities|String|ToString(Float) (Variables|Default|GetFPS)) ";" (LocalVariables|GetDateTimeString)) (Variables|Default|GetLogName))
  (if (Variables|Default|GetCaptureScreenshots)
    (bind _result (Math|Integer|IncrementInt (Variables|Default|GetCurrentFrame))
      (:%20%20
        (if (== (Math|Integer|%(Integer) _result (Variables|Default|GetSkipFrames)) 0)
          (Class|LoggingBlueprintFunctionLibrary|CreateViewportScreenShotFilename (Variables|Default|GetActor) (Utilities|GetScreenshotFilename (LocalVariables|GetNow) (Variables|Default|GetLogName)) (Variables|Default|GetScreenSizeX) (Variables|Default|GetScreenSizeY)))))))

(fn StartLogging
  (bind _returnvalue (Math|DateTime|Now))
  (bind (_year _month _day _hour _minute _second) (Math|DateTime|BreakDateTime _returnvalue))
  (Variables|Default|SetLoggingDone false)
  (Variables|Default|SetIsLogging true)
  (Variables|Default|SetCurrentFrame 0)
  (bind _returnvalue_2 (Utilities|Time|SetTimerbyFunctionName 0 "LogData" (/ 1.0 (Variables|Default|GetLogFrequency)) (Variables|Default|GetIsLogging)))
  (Variables|Default|SetLogTimer _returnvalue_2)
  (bind _output_get (Variables|Default|SetLogName (Utilities|String|Append "LOG_" (Utilities|String|ToString(Integer) _year) "-" (Utilities|String|ToString(Integer) _month) "-" (Utilities|String|ToString(Integer) _day) "_" (Utilities|String|ToString(Integer) _hour) "." (Utilities|String|ToString(Integer) _minute) "." (Utilities|String|ToString(Integer) _second))))
  (Class|LoggingBlueprintFunctionLibrary|AppendLogtoFile "x;y;z;r;p;yw;u_x;u_y;u_z;f_x;f_y;f_z;FPS;TIMESTAMP" _output_get))

(fn StopLogging
  (Variables|Default|SetIsLogging false))

(fn SaveScreenshot
  (Development|ExecuteConsoleCommand (Utilities|String|Append "HighResShot " (Utilities|String|ToString(Integer) (Variables|Default|GetScreenSizeX)) "x" (Utilities|String|ToString(Integer) (Variables|Default|GetScreenSizeY)))))